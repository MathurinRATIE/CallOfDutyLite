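; Lobby game mode that spawns a first-person character for each joining player and controls when the host can start the match.
; On login it cycles through cached PlayerStarts, possesses the new character and tells the game instance to load its save.
; A player count compared to a minimum sets CanStartMatch and shows or hides the start button on the first player controller's lobby widget.
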(event `self.K2_PostLogin`
  (params (NewPlayer :type "PlayerController Object Reference"))
  (`|ExecutionSequence`
    (:`then_0`
      (`/Engine/EditorBlueprintResources/StandardMacros.DoOnce` false
        (:`Completed`
          (bind _outactors (`GameplayStatics.GetAllActorsOfClass` "/Script/Engine.PlayerStart"))
          (set `self.PlayerStarts` _outactors))))
    (:`then_1`
      (if (>= (`self.CurrentPlayerStart`) (`KismetArrayLibrary.Array_Length` (`self.PlayerStarts`)))
        (set `self.CurrentPlayerStart` 0))
      (bind _returnvalue (`|SpawnActorFromClass` "/Game/Game/Global/BP_FirstPersonCharacter.BP_FirstPersonCharacter_C" (`self.GetTransform` (`|GetArrayItem` (`self.PlayerStarts`) (`self.CurrentPlayerStart`))) "Undefined" "MultiplyWithRoot" NewPlayer null))
      (`Controller.Possess` NewPlayer _returnvalue)
      (`/Engine/EditorBlueprintResources/StandardMacros.IncrementInt` (`self.CurrentPlayerStart`)
        (:`  `
          (bind _asgi_game (cast `/Game/Game/Global/GI_Game` (`GameplayStatics.GetGameInstance`)))
          (`/Game/Game/Global/GI_Game.LoadSave` _asgi_game)
          (bind _result (`/Engine/EditorBlueprintResources/StandardMacros.IncrementInt` (`self.PlayerAmount`))
            (:`  `
              (if (>= _result (`self.MinPlayerToStart`))
                (set `self.CanStartMatch` true)
                (`self.ShowStartMatchButton`)))))))))

(event `self.K2_OnLogout`
  (params (ExitingController :type "Controller Object Reference"))
  (bind _result (`/Engine/EditorBlueprintResources/StandardMacros.DecrementInt` (`self.PlayerAmount`))
    (:`  `
      (if (< _result (`self.MinPlayerToStart`))
        (set `self.CanStartMatch` false)
        (bind _aspc_lobby (cast `/Game/Game/Lobby/PC_Lobby` (`GameplayStatics.GetPlayerController` 0)))
        (`Widget.SetVisibility` (`/Game/Game/Lobby/WBP_Lobby.StartMatchButton` (`/Game/Game/Lobby/PC_Lobby.LobbyWidget` _aspc_lobby)) "Collapsed")))))

(event `ShowStartMatchButton`
  (bind _aspc_lobby (cast `/Game/Game/Lobby/PC_Lobby` (`GameplayStatics.GetPlayerController` 0)))
  (`Widget.SetVisibility` (`/Game/Game/Lobby/WBP_Lobby.StartMatchButton` (`/Game/Game/Lobby/PC_Lobby.LobbyWidget` _aspc_lobby)) "Visible"))

(fn `UserConstructionScript`)