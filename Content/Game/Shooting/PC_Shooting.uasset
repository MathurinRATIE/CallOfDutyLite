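; Player controller for the multiplayer shooting mode, handling match start, firing, respawn and match end.
; On possess it disables pawn input and reports ready to PS_Player; countdown completion re-enables input, creating the scoreboard first time and calling GM_Shooting to respawn thereafter.
; Shooting spawns projectiles along the camera rotation, with the player state passed in.
; Match end shows victory or defeat, awards kill-based experience doubled for winners, then the authority server-travels to the lobby.
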(event `self.ReceivePossess`
  (params (PossessedPawn :type "Pawn Object Reference"))
  (`/Engine/EditorBlueprintResources/StandardMacros.DoOnce` false
    (:`Completed`
      (`self.DisableInputs`)
      (bind _asbp_first_person_character (cast `/Game/Game/Global/BP_FirstPersonCharacter` (`self.K2_GetPawn`)))
      (set `self.BP_Character` _asbp_first_person_character)
      (bind _asps_player (cast `/Game/Game/Global/PS_Player` (`self.PlayerState`)))
      (`/Game/Game/Global/PS_Player.PlayerIsReady` _asps_player)
      (if (`self.HasAuthority`)
        _))))

(event `DisableInputs`
  (`self.DisableInput` (`self.K2_GetPawn`) self))

(event `RespawnCountdown`
  (set `/Game/Game/Shooting/WBP_Countdown.State` 3 (stale `StartCountDown` _output_get))
  (`UserWidget.AddToViewport` (stale `StartCountDown` _output_get) 0 :!label _label)
  (`/Game/Game/Shooting/WBP_Countdown.LaunchCountdownAnim` (stale `StartCountDown` _output_get)))

(event `StartCountDown`
  (`/Engine/EditorBlueprintResources/StandardMacros.DoOnce` false
    (:`Completed`
      (bind _returnvalue (`|CreateWidget` "/Game/Game/Shooting/WBP_Countdown.WBP_Countdown_C" self))
      (bind _output_get (set `self.WBP_Countdown` _returnvalue))
      (set `/Game/Game/Shooting/WBP_Countdown.Controller` self _output_get)
      (goto _label))))

(event `CountDownFinished`
  (`self.EnableInput` (`self.K2_GetPawn`) self)
  (`Widget.RemoveFromParent` (`self.WBP_CountDown`))
  (if (not (`self.GameStarted`))
    (set `self.GameStarted` true)
    (bind _returnvalue (`|CreateWidget` "/Game/Game/Shooting/WBP_Scoreboard.WBP_Scoreboard_C" self))
    (bind _output_get (set `self.WBP_ScoreBoard` _returnvalue))
    (`UserWidget.AddToViewport` _output_get 0)
    (`Widget.SetVisibility` (`self.WBP_ScoreBoard`) "Hidden")
    (else
      (`self.Respawn`))))

(event `EnhancedInput|/Game/Game/Inputs/InputActions/IA_Shoot`
  (params (ActionValue :type Boolean) (ElapsedSeconds :type "Float (double-precision)") (TriggeredSeconds :type "Float (double-precision)") (InputAction :type "InputAction Object Reference" :default "/Game/Game/Inputs/InputActions/IA_Shoot.IA_Shoot"))
  (:`Started`
    (if (`self.GameStarted`)
      (`self.Shoot`))))

(event `Shoot`
  (bind _bp_character (`self.BP_Character`))
  (bind _returnvalue (`SceneComponent.K2_GetComponentRotation` (`/Game/Game/Global/BP_FirstPersonCharacter.FirstPersonCamera` _bp_character)))
  (`|SpawnActorFromClass` "/Game/FirstPerson/Blueprints/BP_FirstPersonProjectile.BP_FirstPersonProjectile_C" (`KismetMathLibrary.MakeTransform` (+ (`SceneComponent.K2_GetComponentLocation` (`/Game/Game/Global/BP_FirstPersonCharacter.ShootOrigin` _bp_character)) (`KismetMathLibrary.GreaterGreater_VectorRotator` (`self.Projectile Offset`) _returnvalue)) _returnvalue) "Undefined" "OverrideRootScale" null (`self.PlayerState`) null))

(event `EnhancedInput|/Game/Game/Inputs/InputActions/IA_Scoreboard`
  (params (ActionValue :type Boolean) (ElapsedSeconds :type "Float (double-precision)") (TriggeredSeconds :type "Float (double-precision)") (InputAction :type "InputAction Object Reference" :default "/Game/Game/Inputs/InputActions/IA_Scoreboard.IA_Scoreboard"))
  (bind _wbp_scoreboard (`self.WBP_ScoreBoard`))
  (:`Started`
    (`/Engine/EditorBlueprintResources/StandardMacros.FlipFlop`
      (:`A`
        (`Widget.SetVisibility` _wbp_scoreboard "Visible"))
      (:`B`
        (`Widget.SetVisibility` _wbp_scoreboard "Hidden")))))

(event `Respawn`
  (bind _asgm_shooting (cast `/Game/Game/Shooting/GM_Shooting` (`GameplayStatics.GetGameMode`)))
  (`/Game/Game/Shooting/GM_Shooting.SpawnCharacter` _asgm_shooting self)
  (set `self.BP_Character` (cast `/Game/Game/Global/BP_FirstPersonCharacter` (`self.K2_GetPawn`) :!pure true)))

(event `ShowEndGameBP`
  (bind _asps_player (cast `/Game/Game/Global/PS_Player` (`self.PlayerState`) :!pure true))
  (bind _playerkills (`/Game/Game/Global/PS_Player.PlayerKills` _asps_player))
  (`self.DisableInputs`)
  (`KismetSystemLibrary.Delay` 1.0)
  (bind _asps_player_2 (cast `/Game/Game/Global/PS_Player` (`self.PlayerState`)))
  (bind _returnvalue (`|CreateWidget` "/Game/Game/Shooting/WBP_EndGame.WBP_EndGame_C"))
  (`UserWidget.AddToViewport` _returnvalue 0)
  (if (< (`/Game/Game/Global/PS_Player.PlayerKills` _asps_player_2) (`/Game/Game/Global/GI_Game.VictoryKills` (cast `/Game/Game/Global/GI_Game` (`GameplayStatics.GetGameInstance`) :!pure true)))
    (set `Image.ColorAndOpacity` (struct :`R` 1.0 :`G` 0.170365 :`B` 0.119792 :`A` 1.0) (`/Game/Game/Shooting/WBP_EndGame.Color` _returnvalue))
    (set `TextBlock.Text` "Defeat..." (`/Game/Game/Shooting/WBP_EndGame.Text` _returnvalue)))
  (set `self.WonExperience` (* _playerkills 500))
  (if (>= _playerkills (`/Game/Game/Global/GI_Game.VictoryKills` (cast `/Game/Game/Global/GI_Game` (`GameplayStatics.GetGameInstance`) :!pure true)))
    (bind _output_get (set `self.WonExperience` (* (`self.WonExperience`) 2))))
  (`/Game/Game/Global/PS_Player.AddExperience` _asps_player _output_get)
  (if (`self.HasAuthority`)
    (`KismetSystemLibrary.Delay` 1.0)
    (`KismetSystemLibrary.ExecuteConsoleCommand` "servertravel/Game/Game/Lobby/L_MainLobby?listen" (`GameplayStatics.GetPlayerController` 0))))

(fn `UserConstructionScript`)