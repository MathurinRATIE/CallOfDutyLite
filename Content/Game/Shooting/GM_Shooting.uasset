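; Game mode for the shooting game that spawns and possesses a first-person character for each player on login.
; PostLogin caches all PlayerStart actors once, then runs the same spawn logic as the SpawnCharacter event.
; Spawning cycles through the starts round-robin, wrapping at the end of the list.
; After possession it calls LoadSave on the GI_Game game instance.
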(event `SpawnCharacter`
  (params (PlayerController :type "PlayerController Object Reference"))
  (set `self.PlayerController` PlayerController)
  (if (>= (`self.CurrentPlayerStart`) (`KismetArrayLibrary.Array_Length` (`self.PlayerStarts`))) :!label _label
    (set `self.CurrentPlayerStart` 0))
  (bind _returnvalue (`|SpawnActorFromClass` "/Game/Game/Global/BP_FirstPersonCharacter.BP_FirstPersonCharacter_C" (`self.GetTransform` (`|GetArrayItem` (`self.PlayerStarts`) (`self.CurrentPlayerStart`))) "Undefined" "MultiplyWithRoot" (`self.PlayerController`) null))
  (`Controller.Possess` (`self.PlayerController`) _returnvalue)
  (`/Engine/EditorBlueprintResources/StandardMacros.IncrementInt` (`self.CurrentPlayerStart`)
    (:`  `
      (bind _asgi_game (cast `/Game/Game/Global/GI_Game` (`GameplayStatics.GetGameInstance`)))
      (`/Game/Game/Global/GI_Game.LoadSave` _asgi_game))))

(event `self.K2_PostLogin`
  (params (NewPlayer :type "PlayerController Object Reference"))
  (set `self.PlayerController` NewPlayer)
  (`|ExecutionSequence`
    (:`then_0`
      (`/Engine/EditorBlueprintResources/StandardMacros.DoOnce` false
        (:`Completed`
          (bind _outactors (`GameplayStatics.GetAllActorsOfClass` "/Script/Engine.PlayerStart"))
          (set `self.PlayerStarts` _outactors))))
    (:`then_1`
      (goto _label))))

(fn `UserConstructionScript`)